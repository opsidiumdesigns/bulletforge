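; Example weapon Blueprint for BulletForge that fires bullets and supplies the cosmetic firing effects.
; Fire passes the skeletal mesh's Muzzle socket transform, BulletSettings and the weapon's owner to FireBullet, with debug display on.
; SpawnWeaponEffects plays a fire sound at the actor and spawns a small explosion emitter at the muzzle.
; SpawnShellEffects spawns a small sparks emitter at the Shell socket, standing in for shell ejection.
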(event SpawnWeaponEffects(BP_BulletForgeWeapon)
  (params (Settings :type Ballistics%20Settings%20Object%20Reference))
  (Audio|PlaySoundatLocation "/Game/FPWeapon/Audio/FirstPersonTemplateWeaponFire02.FirstPersonTemplateWeaponFire02" (Transformation|GetActorLocation) "0, 0, 0" 0.5 1.0 0.0 0 0 0 0)
  (Effects|SpawnEmitteratLocation "/Game/StarterContent/Particles/P_Explosion.P_Explosion" (Transformation|GetSocketLocation (Variables|Default|GetSkeletalMesh) "Muzzle") "0, 0, 0" "0.200000,0.200000,0.200000"))

(event SpawnShellEffects(BP_BulletForgeWeapon)
  (params (Settings :type Ballistics%20Settings%20Object%20Reference))
  (bind _skeletalmesh (Variables|Default|GetSkeletalMesh))
  (bind _returnvalue (Transformation|GetSocketTransform _skeletalmesh "Shell" "RTS_World"))
  (bind (_location _rotation) (Math|Transform|BreakTransform _returnvalue))
  (Effects|SpawnEmitteratLocation "/Game/StarterContent/Particles/P_Sparks.P_Sparks" _location _rotation "0.200000,0.200000,0.200000"))

(event Custom|Fire
  (Class|BulletForgeWeaponComponent|FireBullet (Variables|Default|GetBP_BulletForgeWeapon) (Transformation|GetSocketTransform (Variables|Default|GetSkeletalMesh) "Muzzle" "RTS_World") (Variables|Default|GetBulletSettings) (Components|GetOwner) (Utilities|Array|MakeArray) true 5.0))

(fn ConstructionScript)